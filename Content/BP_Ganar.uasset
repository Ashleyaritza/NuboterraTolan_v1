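; Win trigger actor that ends the game when the player enters its Box holding exactly nine keys (Llaves).
; On success it disables input, hides itself and runs a timed, once-only sequence of win widget, fade-out widget and quit.
; Otherwise it briefly shows a missing-keys widget, gated by a DoOnce that resets when the overlap ends.
; Some disconnected leftover logic remains unused in the graph.
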(event `self.ReceiveActorBeginOverlap`
  (params (OtherActor :type "Actor Object Reference")))

(event `self.Box.OnComponentBeginOverlap`
  (params (OverlappedComponent :type "PrimitiveComponent Object Reference") (OtherActor :type "Actor Object Reference") (OtherComp :type "PrimitiveComponent Object Reference") (OtherBodyIndex :type Integer) (bFromSweep :type Boolean) (SweepResult :type "HitResult Structure (by ref)"))
  (bind _asbp_third_person_character (cast `/Game/ThirdPerson/Blueprints/BP_ThirdPersonCharacter` OtherActor))
  (if (== (`/Game/ThirdPerson/Blueprints/BP_ThirdPersonCharacter.Llaves` _asbp_third_person_character) 9)
    (`self.DisableInput` _asbp_third_person_character (`GameplayStatics.GetPlayerController` 0))
    (`self.SetActorHiddenInGame` true)
    (`/Engine/EditorBlueprintResources/StandardMacros.DoOnce` false
      (:`Completed`
        (bind _returnvalue (`|CreateWidget` "/Game/UI/WB_Ganar.WB_Ganar_C" (`GameplayStatics.GetPlayerController` 0)))
        (`UserWidget.AddToViewport` _returnvalue 0)
        (`KismetSystemLibrary.Delay` 3.0)
        (`Widget.RemoveFromParent` _returnvalue)
        (`KismetSystemLibrary.Delay` 1.0)
        (bind _returnvalue_2 (`|CreateWidget` "/Game/UI/WB_FadeOut.WB_FadeOut_C" (`GameplayStatics.GetPlayerController` 0) null))
        (`UserWidget.AddToViewport` _returnvalue_2 0)
        (`WidgetBlueprintLibrary.SetInputMode_UIOnlyEx` (`GameplayStatics.GetPlayerController` 0) null)
        (`KismetSystemLibrary.Delay` 3.0)
        (`KismetSystemLibrary.QuitGame` null "Quit")))
    (else
      (`/Engine/EditorBlueprintResources/StandardMacros.DoOnce` false :!label _label
        (:`Completed`
          (bind _returnvalue_3 (`|CreateWidget` "/Game/UI/WB_FaltanLlaves.WB_FaltanLlaves_C" (`GameplayStatics.GetPlayerController` 0)))
          (set `self.FaltanLlaves` _returnvalue_3)
          (`UserWidget.AddToViewport` _returnvalue_3 0)
          (`KismetSystemLibrary.Delay` 2.0)
          (`Widget.RemoveFromParent` (`self.FaltanLlaves`)))))))

(event `self.Box.OnComponentHit`
  (params (HitComponent :type "PrimitiveComponent Object Reference") (OtherActor :type "Actor Object Reference") (OtherComp :type "PrimitiveComponent Object Reference") (NormalImpulse :type "Vector Structure") (Hit :type "HitResult Structure (by ref)")))

(event `self.Box.OnComponentEndOverlap`
  (params (OverlappedComponent :type "PrimitiveComponent Object Reference") (OtherActor :type "Actor Object Reference") (OtherComp :type "PrimitiveComponent Object Reference") (OtherBodyIndex :type Integer))
  (goto _label :!via `Reset`))

(fn `UserConstructionScript`)